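; Controller for a chat-driven baseball guessing game, holding each user's ID and remaining tries.
; On BeginPlay it finds the Chat_Widget after a short delay and binds to its message event.
; While tries remain, submitted messages spend one and go to BP_BassBallGameMode for relay and checking, otherwise a failure prints.
; Login stores the ID and calls OnUserLogin; HandleVictory only re-fetches the widget.
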(event Custom|GetBroadCast
  (params (UserId :type String))
  (if (Ability|HasAuthority)
    (Development|PrintString UserId)))

(event Custom|OnSendMsgToSever
  (params (Msg :type String))
  (if (<= (Variables|Default|GetRemaingTries) 0)
    (CallFunction|FailText)
    (else
      (Math|Integer|DecrementInt (Variables|Default|GetRemaingTries)
        (:%20%20
          (bind _asbp_bass_ball_game_mode (Utilities|Casting|CastToBP_BassBallGameMode (Game|GetGameMode)))
          (Default|GetMessagefromClient _asbp_bass_ball_game_mode (Utilities|String|Append (Variables|Default|GetUserID) " :  " Msg))
          (Class|BassBallGameMode|CheckBaseBallGame _asbp_bass_ball_game_mode Msg)
          (CallFunction|RemaingNum))))))

(event Custom|FailText
  (Development|PrintString (Utilities|String|Append (Variables|Default|GetUserID) " :  " "기회 소진. 입력불가.")))

(event Custom|OnLoginWithID
  (params (UserId :type String))
  (Default|CallOnUserLogin UserId)
  (Variables|Default|SetUserID UserId))

(event Custom|RemaingNum
  (Development|PrintString (Utilities|String|Append (Variables|Default|GetUserID) " " "남은 횟수" " : " (Utilities|String|ToString(Integer) (Variables|Default|GetRemaingTries)))))

(event Custom|HandleVictory
  (bind _foundwidgets (Widget|GetAllWidgetsOfClass "/Game/BP/Chat_Widget.Chat_Widget_C" true))
  (Variables|Default|SetWidget (Utilities|Array|Get(acopy) _foundwidgets)))

(event EventBeginPlay
  (if (not (Utilities|Enum|Equal(Enum) (Class|Actor|GetRemoteRole) "ROLE_None"))
    (Utilities|FlowControl|Delay 0.5)
    (bind _foundwidgets (Widget|GetAllWidgetsOfClass "/Game/BP/Chat_Widget.Chat_Widget_C" true))
    (bind _output_get (Variables|Default|SetWidget (Utilities|Array|Get(acopy) _foundwidgets)))
    (EventDispatchers|BindEventtoSetMessagetoUserController _output_get (EventDispatchers|CreateEvent :!event Custom|OnSendMsgToSever))))

(fn ConstructionScript)